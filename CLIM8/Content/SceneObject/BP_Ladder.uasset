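; BP_Ladder is a procedural ladder scene object that builds its foot bars in the construction script, with no active gameplay logic.
; It divides LadderLength by FootBarSpread to get a step count, then clears and refills a Hierarchical Instanced Static Mesh with bars stacked along Z.
; When SyncedFootBar is set, it recomputes the spacing from the floored count so the steps divide the length evenly.
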(fn `UserConstructionScript`
  (locals (stepCount :type Integer))
  (bind _output_get (set `local.stepCount` (`KismetMathLibrary.FFloor` (/ (`self.LadderLength`) (`self.FootBarSpread`)))))
  (`InstancedStaticMeshComponent.ClearInstances` (`self.HierarchicalInstancedStaticMesh`))
  (if (`self.SyncedFootBar`)
    (set `self.FootBarSpread` (/ (`self.LadderLength`) _output_get)))
  (for _index (range (`local.stepCount`))
    (`InstancedStaticMeshComponent.AddInstance` (`self.HierarchicalInstancedStaticMesh`) (`KismetMathLibrary.MakeTransform` (`KismetMathLibrary.MakeVector` 0.0 0.0 (* _index (`self.FootBarSpread`)))) false)))