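; BP_GrowCylinder is a scene actor whose Well component is stretched along Z while the player character is climbing.
; BeginPlay caches the player pawn as BP_ThirdPersonCharacter.
; Each Tick checks that character's IsClimbing flag, then sets Well's world transform from the actor's own, interpolating Z scale toward one unit above the actor's current value.
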(event `self.ReceiveBeginPlay`
  (bind _asbp_third_person_character (cast `/Game/ThirdPerson/Blueprints/BP_ThirdPersonCharacter` (`GameplayStatics.GetPlayerPawn` 0)))
  (set `self.Player` _asbp_third_person_character))

(event `self.ReceiveTick`
  (params (DeltaSeconds :type "Float (single-precision)"))
  (bind _returnvalue (`self.GetTransform`))
  (bind _player (`self.Player`))
  (if (and (`KismetSystemLibrary.IsValid` _player) (`/Game/ThirdPerson/Blueprints/BP_ThirdPersonCharacter.IsClimbing` _player))
    (`SceneComponent.K2_SetWorldTransform` (`self.Well`) (`KismetMathLibrary.MakeTransform` (.location _returnvalue) (.rotation _returnvalue) (`KismetMathLibrary.MakeVector` (.x (.scale _returnvalue)) (.y (.scale _returnvalue)) (`KismetMathLibrary.FInterpTo` (.z (.scale _returnvalue)) (+ (.z (.scale _returnvalue)) 1.0) (`GameplayStatics.GetWorldDeltaSeconds`) 4.0))) false false)))

(fn `UserConstructionScript`)